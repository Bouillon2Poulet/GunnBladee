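; Grappling hook projectile for the rifle, with a cable tied to the gun's Muzzle socket.
; It follows the muzzle while stowed, then Shoot shows the cable and launches it with a physics impulse.
; Overlapping hookable terrain or a BP_HookableActor stops it, while hitting a StaticMeshActor counts as a failed hook.
; Dispatchers report each outcome and release, and AttachToGunn hides the cable and re-arms the hook.
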(event OnComponentBeginOverlap(HookComponent)
  (params (OverlappedComponent :type Primitive%20Component%20Object%20Reference) (OtherActor :type Actor%20Object%20Reference) (OtherComp :type Primitive%20Component%20Object%20Reference) (OtherBodyIndex :type Integer) (bFromSweep :type Boolean) (SweepResult :type Hit%20Result%20Structure%20%28by%20ref%29))
  (bind _returnvalue (Utilities|GetClass OtherActor))
  (if (Variables|Default|GetCanAttach)
    (if (Utilities|ClassIsChildOf _returnvalue "/Game/HookableTerain.HookableTerain_C")
      (Physics|SetSimulatePhysics (Variables|Default|GetHookComponent) false)
      (Default|CallOnHookSurface)
      (Development|PrintString "Grab surface !")
      (Variables|Default|SetCanAttach false :!label _label)
      (elif (Utilities|ClassIsChildOf _returnvalue "/Game/BP_HookableActor.BP_HookableActor_C")
        (bind _asbp_hookable_actor (Utilities|Casting|CastToBP_HookableActor OtherActor))
        (Default|Hook _asbp_hookable_actor self)
        (Physics|SetSimulatePhysics (Variables|Default|GetHookComponent) false)
        (Default|CallOnHookActor)
        (Variables|Default|SetIsAttachedToActor true)
        (goto _label)))))

(event OnComponentHit(HookComponent)
  (params (HitComponent :type Primitive%20Component%20Object%20Reference) (OtherActor :type Actor%20Object%20Reference) (OtherComp :type Primitive%20Component%20Object%20Reference) (NormalImpulse :type Vector :default "0, 0, 0") (Hit :type Hit%20Result%20Structure%20%28by%20ref%29))
  (if (== (Utilities|GetClass (.hitactor Hit)) "/Script/Engine.StaticMeshActor")
    (Physics|SetSimulatePhysics (Variables|Default|GetHookComponent) false)
    (Default|CallOnHookFailed)))

(event EventBeginPlay
  (bind _returnvalue (Actor|GetActorOfClass "/Game/FirstPerson/Blueprints/BP_PickUp_Rifle.BP_PickUp_Rifle_C"))
  (Class|CableComponent|SetAttachEndto (Variables|Default|GetCable) _returnvalue "None" "Muzzle"))

(event EventTick
  (params (DeltaSeconds :type Float%20%28single-precision%29))
  (if (Variables|Default|GetIsAttachedToGun)
    (bind _location (Default|GetMuzzleLocation (Variables|Default|GetGun)))
    (Transformation|SetWorldLocation (Variables|Transformation|GetRootComponent) _location false false)))

(fn ConstructionScript)

(fn Shoot
  (params (Direction :type Vector))
  (bind _hookcomponent (Variables|Default|GetHookComponent))
  (Physics|SetSimulatePhysics _hookcomponent true)
  (Physics|AddImpulseatLocation _hookcomponent (* Direction (Variables|Default|GetSpeed)) (Transformation|GetActorLocation) "None")
  (Variables|Default|SetIsAttachedToGun false)
  (Rendering|SetVisibility (Variables|Default|GetCable) true false))

(fn ReleaseActor
  (if (Variables|Default|GetIsAttachedToActor)
    (Default|CallOnReleaseActor)
    (Variables|Default|SetIsAttachedToActor false)))

(fn AttachtoGunn
  (Physics|SetSimulatePhysics (Variables|Default|GetHookComponent) false)
  (Variables|Default|SetIsAttachedToGun true)
  (Rendering|SetVisibility (Variables|Default|GetCable) false false)
  (Default|CallOnReleaseActor)
  (Variables|Default|SetCanAttach true))
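; Gunn power component that launches the player along the camera's forward vector, with strength based on how long the power input is held.
; On BeginPlay it spawns a VFX spawner attached to the weapon's muzzle.
; While input is ongoing, it records elapsed press time and plays VFX.
; On release it applies a velocity-change impulse scaled by that time, starts cooldown, resets the timer and spawns release VFX.
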(event Input|EnhancedActionEvents|EnhancedInputActionIA_GunnPowerReleased
  (params (ActionValue :type Boolean) (ElapsedSeconds :type Float%20%28double-precision%29) (TriggeredSeconds :type Float%20%28double-precision%29) (InputAction :type Input%20Action%20Object%20Reference :default "/Game/FirstPerson/Input/Actions/IA_GunnPowerReleased.IA_GunnPowerReleased"))
  (:Ongoing
    (Variables|Default|SetPressTimer ElapsedSeconds)
    (Default|PlayVFX (Variables|Default|GetVFXSpawner))))

(event EventBeginPlay
  (bind _returnvalue (Game|SpawnActorfromClass "/Game/GunnPowers/BP_VFXSpawner.BP_VFXSpawner_C" (Math|Transform|MakeTransform "0, 0, 0" "0, 0, 0" "1.000000,1.000000,1.000000") "Undefined" "MultiplyWithRoot" 0 0))
  (bind _output_get (Variables|Default|SetVFXSpawner _returnvalue))
  (Transformation|AttachComponentToComponent _output_get (Variables|Default|GetWeaponComponent) "Muzzle" "SnapToTarget" "SnapToTarget" "SnapToTarget" true))

(event EventTick
  (params (DeltaSeconds :type Float%20%28single-precision%29)))

(fn OnPowerActivated
  (|CallParentFunction)
  (Default|SpawnVFX1 (Variables|Default|GetVFXSpawner)))

(fn OnPowerReleased
  (|CallParentFunction)
  (Physics|AddImpulse (Variables|/Script/Engine.Character|GetCharacterMovement (Game|GetPlayerCharacter 0)) (* (Math|Vector|GetForwardVector (Camera|GetCameraRotation (Game|GetPlayerCameraManager 0))) (* (/ (Variables|Default|GetPressTimer) (Variables|Default|GetPressTimerMax)) (Variables|Default|GetMaxImpulsePower))) true)
  (CallFunction|StartCooldown)
  (Variables|Default|SetPressTimer 0.0)
  (Default|SpawnVFX2 (Variables|Default|GetVFXSpawner)))
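; Gunn power component that tracks the cooldown state of a power.
; StartCooldown sets the cooldown flag and fills the timer to its maximum, then Tick counts it down through HandleCooldown while the flag is set.
; When the timer runs out, StopCooldown clears the flag and resets the timer.
; Starting and stopping each call a matching OnStartCooldown or OnStopCooldown dispatcher.
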(event EventBeginPlay)

(event EventTick
  (params (DeltaSeconds :type Float%20%28single-precision%29))
  (if (Variables|Default|GetIsOnCooldown)
    (CallFunction|HandleCooldown DeltaSeconds)))

(fn HandleCooldown
  (params (DeltaSeconds :type Float%20%28double-precision%29))
  (bind _output_get (Variables|Default|SetCooldownTimer (- (Variables|Default|GetCooldownTimer) DeltaSeconds)))
  (if (<= _output_get 0.0)
    (CallFunction|StopCooldown)))

(fn StartCooldown
  (Variables|Default|SetIsOnCooldown true)
  (Variables|Default|SetCooldownTimer (Variables|Default|GetCooldownMax))
  (Default|CallOnStartCooldown))

(fn StopCooldown
  (Variables|Default|SetIsOnCooldown false)
  (Variables|Default|SetCooldownTimer (Variables|Default|GetCooldownMax))
  (Default|CallOnStopCooldown))
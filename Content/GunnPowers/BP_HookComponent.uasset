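; Grappling hook power component for the rifle pickup that spawns a BP_Hook actor and fires it along the camera's aim.
; Tick runs a state machine that moves the hook outward up to a maximum range or reels it back, driven by its hit events.
; A surface hit either impulses the player toward the hook if the button was released, or tethers them within rope length by clamping position.
; Releasing while tethered launches the player along the camera's forward.
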(event Custom|OnHookActor_Event
  (Variables|Default|SetHookState "NewEnumerator2"))

(event Custom|OnHookSucceed_Event
  (if (Utilities|Enum|NotEqual(Enum) (Variables|Default|GetHookState) "NewEnumerator0")
    (if (Variables|Default|GetPlayerHasReleasedButton)
      (CallFunction|ImpulsePawnTowardHook)
      (Variables|Default|SetPlayerHasReleasedButton false)
      (Variables|Default|SetHookState "NewEnumerator2")
      (else
        (CallFunction|AttachPawntoHook)
        (Variables|Default|SetHookState "NewEnumerator3")))))

(event EventBeginPlay
  (bind _asbp_pick_up_rifle (Utilities|Casting|CastToBP_PickUp_Rifle (Components|GetOwner)))
  (bind _returnvalue (Game|SpawnActorfromClass "/Game/GunnPowers/BP_Hook.BP_Hook_C" (Variables|Default|GetGunnMuzzleSpawnTransform) "Undefined" "MultiplyWithRoot" 0 _asbp_pick_up_rifle 0))
  (bind _output_get (Variables|Default|SetHookActor _returnvalue))
  (Physics|SetSimulatePhysics (Variables|/Game/GunnPowers/BP_Hook.BP_Hook_C|GetHookComponent _output_get) false)
  (EventDispatchers|AssignOnHookSurface _output_get (delegate Custom|OnHookSucceed_Event))
  (EventDispatchers|AssignOnHookActor _output_get (delegate Custom|OnHookActor_Event))
  (EventDispatchers|AssignOnHookFailed _output_get (delegate Custom|OnHookActor_Event)))

(event EventTick
  (params (DeltaSeconds :type Float%20%28single-precision%29))
  (switch Utilities|FlowControl|Switch|SwitchonE_HookState (Variables|Default|GetHookState)
    (:NewEnumerator1
      (CallFunction|ShootHook))
    (:NewEnumerator2
      (CallFunction|AttractHook))
    (:NewEnumerator3
      (CallFunction|HandlePawnLocationtoHook))))

(event EventEndPlay
  (params (EndPlayReason :type EEndPlayReason%20Enum :default "Destroyed"))
  (Actor|DestroyActor (Variables|Default|GetHookActor)))

(fn ImpulsePawnTowardHook
  (Development|PrintString "Hello")
  (Physics|AddImpulse (Variables|/Script/Engine.Character|GetCharacterMovement (Game|GetPlayerCharacter 0)) (* (- (Transformation|GetWorldLocation (Variables|/Game/GunnPowers/BP_Hook.BP_Hook_C|GetHookComponent (Variables|Default|GetHookActor))) (Transformation|GetWorldLocation (Variables|/Script/Engine.Character|GetCapsuleComponent (Game|GetPlayerCharacter 0)))) 2.0) true))

(fn AttachPawntoHook
  (Variables|Default|SetHookLength (Math|Vector|VectorLength (- (Transformation|GetActorLocation (Variables|Default|GetHookActor)) (Transformation|GetActorLocation (Game|Player|GetPlayerPawn 0))))))

(fn ShootHook
  (Transformation|AddWorldOffset (Variables|/Script/Engine.Actor|GetRootComponent (Variables|Default|GetHookActor)) (* (Variables|Default|GetShootDirection) (Variables|Default|GetHookSpeed)) true false)
  (CallFunction|HandleHookLength))

(fn HandleHookLength
  (if (> (Math|Vector|VectorLength (- (Transformation|GetWorldLocation (Variables|/Game/GunnPowers/BP_Hook.BP_Hook_C|GetHookComponent (Variables|Default|GetHookActor))) (Transformation|GetWorldLocation (Variables|/Script/Engine.Actor|GetRootComponent (Components|GetOwner))))) 3e+03)
    (Variables|Default|SetHookState "NewEnumerator2")))

(fn AttractHook
  (bind _returnvalue (Components|GetOwner))
  (bind _hookactor (Variables|Default|GetHookActor))
  (bind _hookcomponent (Variables|/Game/GunnPowers/BP_Hook.BP_Hook_C|GetHookComponent _hookactor))
  (bind _rootcomponent (Variables|/Script/Engine.Actor|GetRootComponent _returnvalue))
  (bind _returnvalue_2 (Transformation|GetWorldLocation _hookcomponent))
  (bind _returnvalue_3 (Transformation|GetWorldLocation _rootcomponent))
  (bind _returnvalue_4 (- _returnvalue_3 _returnvalue_2))
  (bind _returnvalue_5 (Math|Vector|VectorLength _returnvalue_4))
  (Transformation|AddWorldOffset _hookcomponent (* (Math|Vector|Normalize _returnvalue_4) (Variables|Default|GetHookSpeed)) true false)
  (if (< _returnvalue_5 5e+01)
    (Variables|Default|SetHookState "NewEnumerator0")
    (Default|AttachtoGunn (Variables|Default|GetHookActor))
    (elif (< _returnvalue_5 1e+02)
      (Default|ReleaseActor (Variables|Default|GetHookActor)))))

(fn HandlePawnLocationtoHook
  (bind _returnvalue (Game|Player|GetPlayerPawn 0))
  (bind _hookactor (Variables|Default|GetHookActor))
  (bind _hooklength (Variables|Default|GetHookLength))
  (bind _returnvalue_2 (Transformation|GetActorLocation _returnvalue))
  (bind _hookcomponent (Variables|/Game/GunnPowers/BP_Hook.BP_Hook_C|GetHookComponent _hookactor))
  (bind _returnvalue_3 (Transformation|GetWorldLocation _hookcomponent))
  (bind _returnvalue_4 (- _returnvalue_2 _returnvalue_3))
  (if (> (Math|Vector|VectorLength _returnvalue_4) _hooklength)
    (Transformation|SetActorLocation (Game|Player|GetPlayerPawn 0) (+ (* (Math|Vector|Normalize _returnvalue_4) _hooklength) _returnvalue_3) false false)))

(fn ImpulsePawnTowardCamera
  (Physics|AddImpulse (Variables|/Script/Engine.Character|GetCharacterMovement (Game|GetPlayerCharacter 0)) (* (Math|Vector|GetForwardVector (Camera|GetCameraRotation (Game|GetPlayerCameraManager 0))) 2.5e+03) true))

(fn OnPowerActivated
  (bind _hookactor (Variables|Default|GetHookActor))
  (|CallParentFunction)
  (if (Utilities|Enum|Equal(Enum) (Variables|Default|GetHookState) "NewEnumerator0")
    (Variables|Default|SetHookState "NewEnumerator1")
    (Variables|Default|SetShootDirection (Math|Rotator|GetRotationXVector (Camera|GetCameraRotation (Game|GetPlayerCameraManager 0))))
    (Variables|/Game/GunnPowers/BP_Hook.BP_Hook_C|SetIsAttachedToGun _hookactor false)
    (Rendering|SetVisibility (Variables|/Game/GunnPowers/BP_Hook.BP_Hook_C|GetCable _hookactor) true false)
    (Variables|/Game/GunnPowers/BP_Hook.BP_Hook_C|SetCanAttach _hookactor true)))

(fn OnPowerReleased
  (|CallParentFunction)
  (if (Utilities|Enum|NotEqual(Enum) (Variables|Default|GetHookState) "NewEnumerator0")
    (Variables|Default|SetPlayerHasReleasedButton true)
    (if (Utilities|Enum|Equal(Enum) (Variables|Default|GetHookState) "NewEnumerator3")
      (CallFunction|ImpulsePawnTowardCamera)
      (Variables|Default|SetHookState "NewEnumerator2")
      (Variables|Default|SetPlayerHasReleasedButton false))))